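; Oil tank Blueprint for the oil rig level that explodes partway through the level timer.
; On BeginPlay it reads the Timer actor's time, halves it into its own countdown and starts a looping one-second timer that decrements it.
; Tick polls the countdown and, once it reaches zero, a DoOnce activates the explosion and smoke particles and fires four radial force impulses.
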(event EventBeginPlay
  (bind _outactors (Actor|GetAllActorsOfClass "/Game/BackgroundItems/timer.timer_C"))
  (Variables|Default|Settime (Math|Float|Truncate (* (Variables|/Game/BackgroundItems/timer.timer_C|GetTime (Utilities|Array|Get(acopy) _outactors)) 0.5)))
  (Utilities|Time|SetTimerbyFunctionName 0 "countDown" 1.0 true))

(event EventTick
  (params (DeltaSeconds :type Float%20%28single-precision%29))
  ;[1 1 1 1 10] Checks if "Time" is zero every tick
  (if (<= (Variables|Default|GetTime) 0)
    (Utilities|FlowControl|DoOnce false
      (:Completed
        (Components|Activation|Activate (Variables|Default|GetP_Explosion) false)
        (Class|RadialForceComponent|FireImpulse (Variables|Default|GetRadialForceCentre))
        (Class|RadialForceComponent|FireImpulse (Variables|Default|GetRadialForceLeft))
        (Class|RadialForceComponent|FireImpulse (Variables|Default|GetRadialForceRight))
        (Class|RadialForceComponent|FireImpulse (Variables|Default|GetRadialForceOuter))
        (Components|Activation|Activate (Variables|Default|Getsmoke) false)))))

(fn ConstructionScript)

(fn CountDown
  ;[1 1 1] The function takes the value of "Time" and reduces it by 1
  (Variables|Default|SetTime (- (Variables|Default|GetTime) 1)))