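; BP_Item_Weapon_Barrel is a barrel weapon item that players can pick up, drop or throw, built on a parent item Blueprint.
; It extends the parent's handlers, switching the static mesh to physics-only collision on pickup.
; Drop and Yeet both restore query-and-physics collision after calling the parent.
; The construction script runs the parent's setup, then sets the barrel's Damage value.
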(event EventBeginPlay
  (|CallParentFunction) ; This node is disabled and will not be called.\nDrag off pins to build functionality.
)

(event Collision|EventActorBeginOverlap
  (params (OtherActor :type Actor%20Object%20Reference)))

(event EventTick
  (params (DeltaSeconds :type Float%20%28single-precision%29))
  (|CallParentFunction DeltaSeconds))

(event EventPickUp
  (params (playerIndex :type Integer%20%28by%20ref%29))
  (|CallParentFunction playerIndex)
  (Collision|SetCollisionEnabled (Variables|Default|GetStaticMesh) "PhysicsOnly"))

(event EventDrop
  (params (playerIndex :type Integer%20%28by%20ref%29))
  (|CallParentFunction playerIndex)
  (Collision|SetCollisionEnabled (Variables|Default|GetStaticMesh) "QueryAndPhysics"))

(event EventYeet
  (params (playerIndex :type Integer) (throwSpeed :type Float%20%28single-precision%29))
  (|CallParentFunction playerIndex throwSpeed)
  (Collision|SetCollisionEnabled (Variables|Default|GetStaticMesh) "QueryAndPhysics"))

(fn ConstructionScript
  (|CallParentFunction)
  (Variables|Default|Setdamage 1e+01))