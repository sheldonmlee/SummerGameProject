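; Base resource point Blueprint that hands a new item to a player whose hands are empty.
; ResoucreCreation first runs MaxCheck, which counts all live actors of ItemClass in the level against MaxAmount.
; Below that cap, it spawns the item at the player's transform and calls the character's InteractWithItem, returning whether the point triggered.
; Child Blueprints are meant to supply the item class and resource ID.
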(event Custom|PickCoolD)

(event EventTick
  (params (DeltaSeconds :type Float%20%28single-precision%29)))

(event EventBeginPlay)

(fn ConstructionScript
  ;[0 0.1145 1] A child BP must be constructed with an specific class and resouceID
  (Variables|Default|SetItemClass (Variables|Default|GetItemClass)))

(fn ResoucreCreation
  (params (playerIndex :type Integer))
  (bind _toomany_ (CallFunction|MaxCheck))
  (if (not _toomany_)
    (bind _asthird_person_character (Utilities|Casting|CastToThirdPersonCharacter (Game|GetPlayerCharacter playerIndex)))
    ;[1 1 1] To see if the player is handling sth
    (Utilities|IsValid (Variables|/Game/ThirdPersonBP/Blueprints/ThirdPersonCharacter.ThirdPersonCharacter_C|GetequippedItem _asthird_person_character)
      (:Is%20Valid
        ;[1 1 1 1 11] return the result of if the Rrsource Point is triggered,
        (bind _output_get (Variables|Default|SetisRPtriggered false))
        (return _output_get))
      (:Is%20Not%20Valid
        ;[1 1 1 1 11] Spawn the target and attach it to the player if player does not have anything in its hand
        (Game|SpawnActorfromClass (Variables|Default|GetItemClass) (Transformation|GetActorTransform _asthird_person_character) "Undefined" 0 0)
        (Default|InteractwithItem _asthird_person_character (Variables|/Game/ThirdPersonBP/Blueprints/ThirdPersonCharacter.ThirdPersonCharacter_C|GetplayerIndexTPC _asthird_person_character))
        (bind _output_get_2 (Variables|Default|SetisRPtriggered true))
        (return _output_get_2)))))

(fn MaxCheck
  (bind _outactors (Actor|GetAllActorsOfClass (Variables|Default|GetItemClass)))
  (if (>= (Utilities|Array|Length _outactors) (Variables|Default|GetmaxAmount))
    (Development|PrintString "Max amount of resources")
    (return true)))