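; Parent Blueprint for interactive items that a ThirdPersonCharacter can pick up and drop, with child Blueprints expected to set item ID and name.
; PickUp finds the character by player index and, if its EquippedItem slot is empty, stores itself there and snaps to the mesh's itemHolder socket.
; Drop detaches the character's equipped item, places it at this item's root transform and clears the slot.
; Both events update CurrentlyEquipped.
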(event EventBeginPlay)

(event EventTick
  (params (DeltaSeconds :type Float%20%28single-precision%29)))

(event EventPickUp
  (params (playerIndex :type Integer%20%28by%20ref%29))
  (bind _returnvalue (Game|GetPlayerCharacter playerIndex))
  ;[1 0.2188 0.2188] pick up
  (bind _asthird_person_character (Utilities|Casting|CastToThirdPersonCharacter _returnvalue))
  (Utilities|IsValid (Variables|/Game/ThirdPersonBP/Blueprints/ThirdPersonCharacter.ThirdPersonCharacter_C|GetequippedItem _asthird_person_character)
    (:Is%20Not%20Valid
      (bind _asthird_person_character_2 (Utilities|Casting|CastToThirdPersonCharacter _returnvalue))
      (Variables|/Game/ThirdPersonBP/Blueprints/ThirdPersonCharacter.ThirdPersonCharacter_C|SetequippedItem _asthird_person_character_2 self)
      (Transformation|AttachComponentToComponent (Variables|/Script/Engine.Character|GetMesh _asthird_person_character_2) "itemHolder" "SnapToTarget" "SnapToTarget" "KeepRelative" true)
      (Variables|Default|SetCurrentlyEquipped? true)
      (Development|PrintString "picked"))))

(event EventDrop
  (params (playerIndex :type Integer%20%28by%20ref%29))
  (bind _defaultsceneroot (Variables|Default|GetDefaultSceneRoot))
  ;[1 0.2396 0.2396] Drop
  (bind _asthird_person_character (Utilities|Casting|CastToThirdPersonCharacter (Game|GetPlayerCharacter playerIndex)))
  (Utilities|IsValid (Variables|/Game/ThirdPersonBP/Blueprints/ThirdPersonCharacter.ThirdPersonCharacter_C|GetequippedItem _asthird_person_character)
    (:Is%20Valid
      (Transformation|DetachFromActor (Variables|/Game/ThirdPersonBP/Blueprints/ThirdPersonCharacter.ThirdPersonCharacter_C|GetequippedItem _asthird_person_character) "KeepWorld" "KeepRelative" "KeepRelative")
      (Transformation|SetActorLocationAndRotation (Variables|/Game/ThirdPersonBP/Blueprints/ThirdPersonCharacter.ThirdPersonCharacter_C|GetequippedItem _asthird_person_character) (Transformation|GetWorldLocation _defaultsceneroot) (Transformation|GetWorldRotation _defaultsceneroot))
      (Variables|/Game/ThirdPersonBP/Blueprints/ThirdPersonCharacter.ThirdPersonCharacter_C|SetequippedItem _asthird_person_character 0)
      (Variables|Default|SetCurrentlyEquipped? false)
      (Development|PrintString "drop"))))

(fn ConstructionScript
  ;[0.1299 0.1558 1] A child BP must construct itemID &itemName
)